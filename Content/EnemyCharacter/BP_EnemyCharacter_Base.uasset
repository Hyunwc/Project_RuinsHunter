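; Base Blueprint for enemy characters that handles what happens when an enemy dies.
; OnEnemyDied pauses mesh animation and disables capsule collision, then async-loads the supplied dissolve Niagara system.
; Once loaded, it attaches the effect to the mesh, destroys the combat component's equipped weapon and removes the actor after a short delay.
; Hit-material and dissolve-color nodes are present but unconnected.
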(event EventBeginPlay)

(event Collision|EventActorBeginOverlap
  (params (OtherActor :type Actor%20Object%20Reference)))

(event EventTick
  (params (DeltaSeconds :type Float%20%28single-precision%29)))

(event EventOnEnemyDied
  (params (DissolveNiagaraSystem :type Niagara%20System%20Soft%20Object%20Reference))
  (bind _enemycombatcomponent (Variables|Default|GetEnemyCombatComponent))
  (bind _returnvalue (Class|PawnCombatComponent|GetCharacterCurrentEquippedWeapon _enemycombatcomponent))
  (Utilities|FlowControl|Sequence
    (:then_0
      (Variables|/Script/Engine.SkeletalMeshComponent|SetbPauseAnims (Variables|Character|GetMesh) true)
      (Collision|SetCollisionEnabled (Variables|Default|GetCapsuleComponent) "NoCollision"))
    (:then_1
      (bind _object (Utilities|AsyncLoadAsset DissolveNiagaraSystem)
        (:Completed
          (bind _asniagara_system (Utilities|Casting|CastToNiagaraSystem _object))
          (Niagara|SpawnSystemAttached _asniagara_system (Variables|Character|GetMesh) "None" "0, 0, 0" "0, 0, 0" "KeepRelativeOffset" true)
          ;[0 0 0] 무기가 유효할 경우 파괴
          (Utilities|IsValid _returnvalue
            (:Is%20Valid
              (Actor|DestroyActor _returnvalue))
            (:Is%20Not%20Valid
              _))
          (Utilities|FlowControl|Delay 3.0)
          (Actor|DestroyActor))))))

(fn ConstructionScript)